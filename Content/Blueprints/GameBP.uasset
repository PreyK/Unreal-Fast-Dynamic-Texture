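; GameBP is a touch drawing actor that shows a runtime canvas through an orthographic camera it sets as the view target.
; It constructs a DrawingCanvasBP object, feeds its texture into a dynamic material on a scaled Canvas component, and updates it every Tick.
; Touch press and move deproject to world XY and draw dots at changed pixel coordinates.
; Debug keys clear the canvas or toggle full versus chunked region updates.
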(event EventBeginPlay
  (Development|ExecuteConsoleCommand "viewmode unlit" 0)
  (Game|Player|SetViewTargetwithBlend (Game|GetPlayerController 0) self 0.0 "VTBlend_Linear" 0.0 false) ; Setup Camera
  (CallFunction|InitializeDrawingCanvas))

(event EventTick
  (params (DeltaSeconds :type Float%20%28single-precision%29))
  (Class|DrawingCanvas|UpdateCanvas (Variables|Default|GetDrawingCanvas)))

(event Input|KeyboardEvents|SpaceBar
  (params (Key :type Key%20Structure :default "None"))
  (bind _drawingcanvas (Variables|Default|GetDrawingCanvas))
  (:Pressed
    (bind _output_get (Variables|/Script/Tutorial_Canvas.DrawingCanvas|SetUpdateFullRegion _drawingcanvas (not (Variables|/Script/Tutorial_Canvas.DrawingCanvas|GetUpdateFullRegion _drawingcanvas))))
    (if _output_get
      (Development|PrintString "Updating full region....")
      (else
        (Development|PrintString "Updating chunked region....")))))

(event Input|KeyboardEvents|C
  (params (Key :type Key%20Structure :default "None"))
  (:Pressed
    (Class|DrawingCanvas|ClearCanvas (Variables|Default|GetDrawingCanvas))))

(event Input|KeyboardEvents|U
  (params (Key :type Key%20Structure :default "None")))

(event Input|TouchEvents|InputTouch
  (params (Location :type Vector) (FingerIndex :type ETouchIndex%20Enum))
  (bind (_coordx _coordy) (CallFunction|GetTouchCoords Location))
  (bind _canvaswidth (Variables|Default|GetCanvasWidth))
  (bind _canvasheight (Variables|Default|GetCanvasHeight))
  (bind _returnvalue (/ _canvasheight 2))
  (bind _returnvalue_2 (/ _canvaswidth 2))
  (bind _returnvalue_3 (Math|Conversions|ToFloat(Integer) _returnvalue_2))
  (bind _returnvalue_4 (Math|Conversions|ToFloat(Integer) _returnvalue))
  (bind _returnvalue_5 (+ _coordy _returnvalue_4))
  (bind _returnvalue_6 (+ _coordx _returnvalue_3))
  (bind _returnvalue_7 (Math|Float|Round _returnvalue_6))
  (bind _returnvalue_8 (Math|Float|Round _returnvalue_5))
  (:Pressed
    (if (or (!= (Variables|Default|GetCurrentMouseX) _returnvalue_7) (!= (Variables|Default|GetCurrentMouseY) _returnvalue_8)) :!label _label
      (bind _output_get (Variables|Default|SetCurrentMouseX _returnvalue_7))
      (bind _output_get_2 (Variables|Default|SetCurrentMouseY _returnvalue_8))
      (Class|DrawingCanvas|DrawDot (Variables|Default|GetDrawingCanvas) _output_get _output_get_2 210)))
  (:Released
    (Variables|Default|SetCurrentMouseX -1)
    (Variables|Default|SetCurrentMouseY -1))
  (:Moved
    (goto _label)))

(fn ConstructionScript)

(fn InitializeDrawingCanvas
  ;[0 0.02604 0.01004] Init Drawing Canvas Object
  (bind _returnvalue (Game|ConstructObjectfromClass self "/Game/Blueprints/DrawingCanvasBP.DrawingCanvasBP_C"))
  (Variables|Default|SetDrawingCanvas _returnvalue)
  (bind _returnvalue_2 (Class|DrawingCanvas|InitializeCanvas (Variables|Default|GetDrawingCanvas) (Variables|Default|GetCanvasWidth) (Variables|Default|GetCanvasHeight) 4))
  (Class|DrawingCanvas|InitializeDrawingTools (Variables|Default|GetDrawingCanvas) 100)
  ;[0 0.01121 0.04167] Init Drawing Canvas Material
  (bind _returnvalue_3 (Rendering|Material|CreateDynamicMaterialInstance (Variables|Default|GetCanvas) 0 0 "None" :!class /Script/Engine.PrimitiveComponent))
  (Variables|Default|SetCanvasMID _returnvalue_3)
  (Rendering|Material|SetTextureParameterValue (Variables|Default|GetCanvasMID) "TextureInput" _returnvalue_2)
  ;[0 0.01121 0.04167] Init Scene Objects
  (Transformation|SetRelativeScale3D (Variables|Default|GetCanvas) (Math|Vector|MakeVector (Math|Conversions|ToFloat(Integer) (/ (Variables|Default|GetCanvasWidth) 100)) (Math|Conversions|ToFloat(Integer) (/ (Variables|Default|GetCanvasHeight) 100)) 0.0))
  (Class|CameraComponent|SetOrthoWidth (Variables|Default|GetCamera) (Math|Conversions|ToFloat(Integer) (Variables|Default|GetCanvasWidth))))

(fn GetTouchCoords
  (params (InputTouchLocation :type Vector))
  (bind (_x _y) (Math|Vector|BreakVector InputTouchLocation))
  (bind _returnvalue (Game|GetPlayerController 0))
  (bind _worldlocation (Class|PlayerController|DeprojectScreenPositiontoWorld _returnvalue _x _y))
  (bind (_x_2 _y_2) (Math|Vector|BreakVector _worldlocation))
  (return _x_2 _y_2))